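; Game instance for Toon Tanks that holds the selected difficulty and provides functions to host or join multiplayer games.
; Four setters act as a radio switch over the Starter, Intermediate, Experienced and MasterMind booleans, leaving only one true.
; Hosting builds an open console command with the listen option, while joining issues open commands for the level, then the IP address.
; Both network functions print a success message without checking the result.
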(fn SetDifficultytoStarter
  (Utilities|FlowControl|Sequence
    (:then_0
      (Variables|Default|SetStarterDifficulty true))
    (:then_1
      (Variables|Default|SetIntermediateDifficulty false))
    (:then_2
      (Variables|Default|SetExperiencedDifficulty false))
    (:then_3
      (Variables|Default|SetMasterMindDifficulty false))))

(fn SetDifficultytoIntermediate
  (Variables|Default|SetStarterDifficulty false)
  (Variables|Default|SetIntermediateDifficulty true)
  (Variables|Default|SetExperiencedDifficulty false)
  (Variables|Default|SetMasterMindDifficulty false))

(fn SetDifficultytoExperienced
  (Variables|Default|SetStarterDifficulty false)
  (Variables|Default|SetIntermediateDifficulty false)
  (Variables|Default|SetExperiencedDifficulty true)
  (Variables|Default|SetMasterMindDifficulty false))

(fn SetDifficultytoMasterMind
  (Utilities|FlowControl|Sequence
    (:then_0
      (Variables|Default|SetStarterDifficulty false))
    (:then_1
      (Variables|Default|SetIntermediateDifficulty false))
    (:then_2
      (Variables|Default|SetExperiencedDifficulty false))
    (:then_3
      (Variables|Default|SetMasterMindDifficulty true))))

(fn HostMultiplayer
  (params (LevelName :type String))
  (Development|ExecuteConsoleCommand (Utilities|String|Append "open " LevelName "?listen") 0)
  (Development|PrintString "host success"))

(fn JoinMultiplayer
  (params (IP%20Address :type String) (Level%20Name :type String))
  (Development|ExecuteConsoleCommand (Utilities|String|Append "open " Level%20Name) (Game|GetPlayerController 0))
  (Development|ExecuteConsoleCommand (Utilities|String|Append "open " IP%20Address) 0)
  (Development|PrintString "JoinedServer Success"))