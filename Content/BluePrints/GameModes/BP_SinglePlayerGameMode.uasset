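; Single-player game mode for Toon Tanks that shows the start and end widgets and handles the level result.
; GameOver records the win or loss in ToonTanksGameInstance, then opens MainMenu after a short delay.
; ApplyDifficulty, not called here, casts TurretRef to both turret types and sets fire range and rate from the instance's difficulty flags.
; TargetArrowsCoordinates projects a target's direction to compute a margin-inset screen-edge position and angle.
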(event EventGameOver
  (params (PlayerWon :type Boolean))
  (Variables|Default|SetPlayerBeatLevel PlayerWon)
  (bind _returnvalue (UserInterface|CreateWidget "/Game/Widgets/WBP_GameEnd.WBP_GameEnd_C"))
  (Default|SetPlayerWon _returnvalue PlayerWon)
  (UserInterface|Viewport|AddtoViewport _returnvalue 0)
  (bind _astoon_tanks_game_instance (Utilities|Casting|CastToToonTanksGameInstance (Game|GetGameInstance)))
  (if (Variables|Default|GetPlayerBeatLevel)
    ;[1 1 1] player beat the level
    (Variables|/Game/BluePrints/GameInstances/ToonTanksGameInstance.ToonTanksGameInstance_C|SetPlayerBeatCurrentLevel _astoon_tanks_game_instance (Variables|Default|GetPlayerBeatLevel))
    (else
      ;[1 1 1] player lost the level
      (Variables|/Game/BluePrints/GameInstances/ToonTanksGameInstance.ToonTanksGameInstance_C|SetPlayerBeatCurrentLevel _astoon_tanks_game_instance (Variables|Default|GetPlayerBeatLevel))))
  (Variables|/Game/BluePrints/GameInstances/ToonTanksGameInstance.ToonTanksGameInstance_C|SetPlayerFinishedGame _astoon_tanks_game_instance true)
  (Utilities|FlowControl|Delay 2.5)
  (Game|OpenLevel(byName) "MainMenu"))

(event EventGameStart
  (bind _returnvalue (UserInterface|CreateWidget "/Game/Widgets/WBP_GameStart.WBP_GameStart_C"))
  (Default|SetStartDelay _returnvalue (Variables|Default|GetStartDelay))
  (UserInterface|Viewport|AddtoViewport _returnvalue 0))

(fn ConstructionScript)

(fn ApplyDifficulty
  (bind _astoon_tanks_game_instance (Utilities|Casting|CastToToonTanksGameInstance (Game|GetGameInstance)))
  (Utilities|FlowControl|Sequence
    (:then_0
      (bind _asbp_pawn_turret (Utilities|Casting|CastToBP_PawnTurret (Variables|Default|GetTurretRef))))
    (:then_1
      (bind _asbp_big_turret (Utilities|Casting|CastToBP_BigTurret (Variables|Default|GetTurretRef))))
    (:then_2
      (if (Variables|/Game/BluePrints/GameInstances/ToonTanksGameInstance.ToonTanksGameInstance_C|GetStarterDifficulty _astoon_tanks_game_instance)
        (Utilities|FlowControl|Sequence
          (:then_0
            (Variables|/Script/ToonTanks.PawnTurret|SetFireRange _asbp_pawn_turret 1.0)
            (Variables|/Script/ToonTanks.PawnTurret|SetFireRange _asbp_big_turret 1.0))
          (:then_1
            (Variables|/Script/ToonTanks.PawnTurret|SetFireRate _asbp_pawn_turret 1.0)
            (Variables|/Script/ToonTanks.PawnTurret|SetFireRate _asbp_big_turret 1.0)))
        (elif (Variables|/Game/BluePrints/GameInstances/ToonTanksGameInstance.ToonTanksGameInstance_C|GetIntermediateDifficulty _astoon_tanks_game_instance)
          (Utilities|FlowControl|Sequence
            (:then_0
              (Variables|/Script/ToonTanks.PawnTurret|SetFireRange _asbp_pawn_turret 2.0)
              (Variables|/Script/ToonTanks.PawnTurret|SetFireRange _asbp_big_turret 7.5e+02))
            (:then_1
              (Variables|/Script/ToonTanks.PawnTurret|SetFireRate _asbp_pawn_turret 2.0)
              (Variables|/Script/ToonTanks.PawnTurret|SetFireRate _asbp_big_turret 2.0)))
          (elif (Variables|/Game/BluePrints/GameInstances/ToonTanksGameInstance.ToonTanksGameInstance_C|GetExperiencedDifficulty _astoon_tanks_game_instance)
            (Utilities|FlowControl|Sequence
              (:then_0
                (Variables|/Script/ToonTanks.PawnTurret|SetFireRange _asbp_pawn_turret 0.0)
                (Variables|/Script/ToonTanks.PawnTurret|SetFireRange _asbp_big_turret 0.0))
              (:then_1
                (Variables|/Script/ToonTanks.PawnTurret|SetFireRate _asbp_pawn_turret 0.0)
                (Variables|/Script/ToonTanks.PawnTurret|SetFireRate _asbp_big_turret 0.0)))
            (elif (Variables|/Game/BluePrints/GameInstances/ToonTanksGameInstance.ToonTanksGameInstance_C|GetMasterMindDifficulty _astoon_tanks_game_instance)
              (Utilities|FlowControl|Sequence
                (:then_0
                  (Variables|/Script/ToonTanks.PawnTurret|SetFireRange _asbp_pawn_turret 0.0)
                  (Variables|/Script/ToonTanks.PawnTurret|SetFireRange _asbp_big_turret 0.0))
                (:then_1
                  (Variables|/Script/ToonTanks.PawnTurret|SetFireRate _asbp_pawn_turret 0.0)
                  (Variables|/Script/ToonTanks.PawnTurret|SetFireRate _asbp_big_turret 0.0))))))))))

(fn TargetArrowsCoordinates
  (params (Target :type Vector) (Margin :type Float%20%28single-precision%29))
  (bind _returnvalue (Game|GetPlayerController 0))
  (bind (_sizex _sizey) (HUD|GetViewportSize _returnvalue))
  (bind _returnvalue_2 (* _sizey 0.5))
  (bind _returnvalue_3 (* _sizex 0.5))
  (bind (_worldlocation _worlddirection) (Class|PlayerController|DeprojectScreenPositiontoWorld _returnvalue _returnvalue_3 _returnvalue_2))
  (bind _returnvalue_4 (* _worlddirection 1e+01))
  (bind _returnvalue_5 (+ _worldlocation _returnvalue_4))
  (bind _returnvalue_6 (Math|Rotator|FindLookatRotation Target _returnvalue_5))
  (bind _returnvalue_7 (Math|Vector|GetForwardVector _returnvalue_6))
  (bind _returnvalue_8 (+ _returnvalue_7 _returnvalue_5))
  (bind _screenlocation (Class|PlayerController|ProjectWorldLocationtoScreen _returnvalue _returnvalue_8 false))
  (bind (_x _y) (Math|Vector2D|BreakVector2D _screenlocation))
  ;[1 1 1] invert Margin
  (Variables|Default|SetMarginValue (- 1.0 Margin))
  (Variables|Default|SetHalfScreenWidth _returnvalue_3)
  (Variables|Default|SetHalfScreenHeight _returnvalue_2)
  (return (+ (Variables|Default|GetHalfScreenWidth) (* (Variables|Default|GetMarginValue) (* (Math|Float|Absolute(Float) (/ (Variables|Default|GetHalfScreenWidth) (/ (- _y (Variables|Default|GetHalfScreenHeight)) (Math|Float|Absolute(Float) (+ (- _x (Variables|Default|GetHalfScreenWidth)) (- _y (Variables|Default|GetHalfScreenHeight))))))) (Math|Float|Min(Float) (Math|Float|Absolute(Float) (/ (Variables|Default|GetHalfScreenWidth) (/ (- _y (Variables|Default|GetHalfScreenHeight)) (Math|Float|Absolute(Float) (+ (- _x (Variables|Default|GetHalfScreenWidth)) (- _y (Variables|Default|GetHalfScreenHeight))))))) (Math|Float|Absolute(Float) (/ (Variables|Default|GetHalfScreenHeight) (/ (- _y (Variables|Default|GetHalfScreenHeight)) (Math|Float|Absolute(Float) (+ (- _x (Variables|Default|GetHalfScreenWidth)) (- _y (Variables|Default|GetHalfScreenHeight))))))))))) (+ (Variables|Default|GetHalfScreenHeight) (* (Variables|Default|GetMarginValue) (* (Math|Float|Min(Float) (Math|Float|Absolute(Float) (/ (Variables|Default|GetHalfScreenWidth) (/ (- _y (Variables|Default|GetHalfScreenHeight)) (Math|Float|Absolute(Float) (+ (- _x (Variables|Default|GetHalfScreenWidth)) (- _y (Variables|Default|GetHalfScreenHeight))))))) (Math|Float|Absolute(Float) (/ (Variables|Default|GetHalfScreenHeight) (/ (- _y (Variables|Default|GetHalfScreenHeight)) (Math|Float|Absolute(Float) (+ (- _x (Variables|Default|GetHalfScreenWidth)) (- _y (Variables|Default|GetHalfScreenHeight)))))))) (Math|Float|Absolute(Float) (/ (Variables|Default|GetHalfScreenHeight) (/ (- _y (Variables|Default|GetHalfScreenHeight)) (Math|Float|Absolute(Float) (+ (- _x (Variables|Default|GetHalfScreenWidth)) (- _y (Variables|Default|GetHalfScreenHeight)))))))))) (Class|KismetMathLibrary|DegAtan2 (/ (Variables|Default|GetHalfScreenWidth) (/ (- _y (Variables|Default|GetHalfScreenHeight)) (Math|Float|Absolute(Float) (+ (- _x (Variables|Default|GetHalfScreenWidth)) (- _y (Variables|Default|GetHalfScreenHeight)))))) (/ (Variables|Default|GetHalfScreenHeight) (/ (- _y (Variables|Default|GetHalfScreenHeight)) (Math|Float|Absolute(Float) (+ (- _x (Variables|Default|GetHalfScreenWidth)) (- _y (Variables|Default|GetHalfScreenHeight)))))))))